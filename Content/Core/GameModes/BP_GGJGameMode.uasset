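; Game mode that acts as a clock for the game, broadcasting a periodic transmission pulse through the OnTransmissionPulse event dispatcher.
; Tick adds each frame's delta, converted to whole milliseconds to limit truncation loss, to an elapsed Timespan.
; When that total reaches DelayBetweenSignals, it resets to zero, discarding any overshoot, and fires the pulse.
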(event EventBeginPlay)

(event EventTick
  (params (DeltaSeconds :type Float%20%28single-precision%29))
  (if (>= (+ (Variables|Default|GetElapsedTimeSinceLastSignal) (Math|Timespan|MakeTimespan 0 0 0 0 (Math|Float|Truncate (* DeltaSeconds 1e+03)))) (Variables|Default|GetDelayBetweenSignals))
    (Variables|Default|SetElapsedTimeSinceLastSignal (Math|Timespan|MakeTimespan 0))
    (Default|CallOnTransmissionPulse)
    (else
      (Variables|Default|SetElapsedTimeSinceLastSignal (+ (Variables|Default|GetElapsedTimeSinceLastSignal) (Math|Timespan|MakeTimespan 0 0 0 0 (Math|Float|Truncate (* DeltaSeconds 1e+03))))))))

(fn ConstructionScript)