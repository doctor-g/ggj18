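; BP_Transmitter is an actor that broadcasts the command selected on its console as a signal.
; On BeginPlay it binds to the GGJ game mode's transmission pulse event.
; Each pulse reads CurrentCommand from the WBP_CommandConsole in its Controls widget component and, unless one specific enum value is selected, spawns a BP_Signal of that type at the transmitter's transform.
; Hit and cursor-over events on Controls only print debug strings.
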(event OnComponentHit(Controls)
  (params (HitComponent :type Primitive%20Component%20Object%20Reference) (OtherActor :type Actor%20Object%20Reference) (OtherComp :type Primitive%20Component%20Object%20Reference) (NormalImpulse :type Vector :default "0, 0, 0") (Hit :type Hit%20Result%20Structure%20%28by%20ref%29))
  (Development|PrintString "Component hit"))

(event OnBeginCursorOver(Controls)
  (params (TouchedComponent :type Primitive%20Component%20Object%20Reference))
  (Development|PrintString "Mouseover"))

(event Custom|OnTransmissionPulse
  (bind _aswbp_command_console (Utilities|Casting|CastToWBP_CommandConsole (UserInterface|GetUserWidgetObject (Variables|Default|GetControls))))
  (if (Utilities|Enum|NotEqual(Enum) (Variables|/Game/Characters/WBP_CommandConsole.WBP_CommandConsole_C|GetCurrentCommand _aswbp_command_console) "NewEnumerator3")
    (Game|SpawnActorfromClass "/Game/Characters/BP_Signal.BP_Signal_C" (Transformation|GetActorTransform) "Undefined" 0 (Variables|/Game/Characters/WBP_CommandConsole.WBP_CommandConsole_C|GetCurrentCommand _aswbp_command_console) 0)))

(event EventBeginPlay
  (bind _gamemode (Utilities|GetGGJGameMode)
    (:Done
      (EventDispatchers|BindEventtoOnTransmissionPulse _gamemode (delegate Custom|OnTransmissionPulse)))))

(event Collision|EventActorBeginOverlap
  (params (OtherActor :type Actor%20Object%20Reference)))

(event EventTick
  (params (DeltaSeconds :type Float%20%28single-precision%29)))

(fn ConstructionScript)