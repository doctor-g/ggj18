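; BP_Signal is a directional command signal (forward, forward-left/right, stop, backward) that homes in on the player's drone via physics velocity each tick.
; A looping timer rolls against age times glitch chance, glitching only when the random value is higher, so glitches become rarer with age.
; A glitch randomizes the signal type, then a timeline flickers random sprites with degrade sounds before settling on the matching sprite.
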(event Custom|OnGlitchTimer
  (if (< (* (Variables|Default|GetSecondsAlive) (Variables|Default|GetGlitchChancePerSecond)) (Math|Random|RandomFloat))
    (CallFunction|SetRandomSignalType)
    (Timeline|Timeline_0 PlayFromStart
      (:Finished
        ;[1 1 1] End on proper sprite
        (CallFunction|UpdateSprite))
      (:Glitch
        ;[1 1 1] Glitch to random sprites
        (bind _sprite (CallFunction|GetRandomSprite))
        (Rendering|Components|Sprite|SetSprite (Variables|Default|GetSprite) _sprite)
        (Audio|PlaySound2D "/Game/Characters/A_Degrade.A_Degrade")))))

(event EventBeginPlay
  (Utilities|Time|SetTimerbyEvent (delegate Custom|OnGlitchTimer) 1.2 true)
  (CallFunction|UpdateSprite))

(event Collision|EventActorBeginOverlap
  (params (OtherActor :type Actor%20Object%20Reference)))

(event EventTick
  (params (DeltaSeconds :type Float%20%28single-precision%29))
  (bind _sprite (Variables|Default|GetSprite))
  (Utilities|FlowControl|Sequence
    (:then_0
      ;[1 1 1] Move signal sprite toward the drone
      (bind _asbp_drone (Utilities|Casting|CastToBP_Drone (Pawn|GetControlledPawn (Game|GetPlayerController 0))))
      (Physics|SetPhysicsLinearVelocity _sprite (Math|Vector|RotateVector (Math|Vector|MakeVector (Variables|Default|GetSignalSpeed) 0.0 0.0) (Math|Rotator|FindLookatRotation (Transformation|GetWorldLocation _sprite) (Transformation|GetWorldLocation (Variables|/Game/Characters/BP_Drone.BP_Drone_C|GetSprite _asbp_drone)))) false "None"))
    (:then_1
      (Variables|Default|SetSecondsAlive (+ DeltaSeconds (Variables|Default|GetSecondsAlive))))))

(fn ConstructionScript)

(fn SetRandomSignalType
  (Variables|Default|SetSignalType (Utilities|Enum|ByteToEnumESignalType (Math|Conversions|ToByte(Integer) (Math|Random|RandomIntegerinRange 1 (- (|GetNumEnumEntries) 1))))))

(fn UpdateSprite
  (bind _sprite (Variables|Default|GetSprite))
  (switch Utilities|FlowControl|Switch|SwitchonESignalType (Variables|Default|GetSignalType)
    (:NewEnumerator3
      (Development|PrintString "CANNOT HAVE A NONE SIGNAL SPRITE"))
    (:NewEnumerator0
      (Rendering|Components|Sprite|SetSprite _sprite "/Game/Characters/SPR_Forward.SPR_Forward"))
    (:NewEnumerator1
      (Rendering|Components|Sprite|SetSprite _sprite "/Game/Characters/SPR_ForwardLeft.SPR_ForwardLeft"))
    (:NewEnumerator2
      (Rendering|Components|Sprite|SetSprite _sprite "/Game/Characters/SPR_ForwardRight.SPR_ForwardRight"))
    (:NewEnumerator4
      (Rendering|Components|Sprite|SetSprite _sprite "/Game/Characters/SPR_Stop.SPR_Stop"))
    (:NewEnumerator5
      (Rendering|Components|Sprite|SetSprite _sprite "/Game/Characters/SPR_Backward.SPR_Backward"))))

(fn GetRandomSprite
  (bind _signalsprites (Variables|Default|GetSignalSprites))
  (return (Utilities|Array|Get(acopy) _signalsprites (Math|Random|RandomIntegerinRange 0 (- (Utilities|Array|Length _signalsprites) 1)))))